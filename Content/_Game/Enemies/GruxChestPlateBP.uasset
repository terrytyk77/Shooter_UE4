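; GruxChestPlateBP is an enemy Blueprint that supplies the health bar and floating hit-number UI on top of its parent class.
; On BeginPlay it binds itself to the EnemyHealthBP widget and hides it, then show and hide events toggle visibility.
; ShowHitNumber spawns an animated damage widget with a headshot flag, projects the hit location to screen space, and passes it to StoreHitNumber for tracking.
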(event EventBeginPlay
  (|CallParentFunction)
  (bind _asenemy_health_bp (Utilities|Casting|CastToEnemyHealthBP (UserInterface|GetUserWidgetObject (Variables|Default|GetHealthBar))))
  (Variables|/Game/_Game/HUD/EnemyHealthBP.EnemyHealthBP_C|SetEnemy _asenemy_health_bp self)
  (Widget|SetVisibility (UserInterface|GetUserWidgetObject (Variables|Default|GetHealthBar)) "Hidden"))

(event EventShowHitNumber
  (params (Damage :type Integer) (HitLocation :type Vector :default "0, 0, 0") (bHeadShot :type Boolean))
  (bind _returnvalue (UserInterface|CreateWidget "/Game/_Game/HUD/HitNumber.HitNumber_C"))
  (Variables|/Game/_Game/HUD/HitNumber.HitNumber_C|SetHitText _returnvalue (Utilities|Text|ToText(Integer) Damage))
  (Variables|/Game/_Game/HUD/HitNumber.HitNumber_C|SetHeadShot _returnvalue bHeadShot)
  (UserInterface|Viewport|AddtoViewport _returnvalue 0)
  (UserInterface|Animation|PlayAnimation _returnvalue (Variables|/Game/_Game/HUD/HitNumber.HitNumber_C|GetHitNumberAnimation _returnvalue) 0.0 1 "Forward" 1.0 false)
  (Class|UserWidget|SetPositioninViewport _returnvalue (.ScreenPosition (Class|GameplayStatics|ProjectWorldtoScreen (Game|GetPlayerController 0) HitLocation false)) true)
  (Class|Enemy|StoreHitNumber _returnvalue HitLocation))

(event EventShowHealthBar
  (Widget|SetVisibility (UserInterface|GetUserWidgetObject (Variables|Default|GetHealthBar)) "Visible")
  (|CallParentFunction))

(event EventHideHealthBar
  (Widget|SetVisibility (UserInterface|GetUserWidgetObject (Variables|Default|GetHealthBar)) "Hidden"))

(fn ConstructionScript)